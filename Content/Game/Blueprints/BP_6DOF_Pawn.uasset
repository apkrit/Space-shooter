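; Player-controlled pawn for free-flight movement, driven by physics on its BodyMesh.
; MoveForward and MoveRight axis inputs add linear velocity along the actor's forward and right vectors every frame, without delta-time scaling.
; LookUp and Turn apply pitch and yaw as local rotations, so steering follows the pawn's current orientation.
; Despite the 6DOF name, it has no roll or vertical-thrust input.
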(event `self.ReceiveBeginPlay`)

(event `self.ReceiveActorBeginOverlap`
  (params (OtherActor :type "Actor Object Reference")))

(event `InputAxis|MoveForward`
  (params (AxisValue :type "Float (single-precision)"))
  (`PrimitiveComponent.SetPhysicsLinearVelocity` (`self.BodyMesh`) (* (`KismetMathLibrary.GetForwardVector` (`self.K2_GetActorRotation`)) (* AxisValue 30.0)) true "None"))

(event `self.ReceiveTick`
  (params (DeltaSeconds :type "Float (single-precision)")))

(event `InputAxis|MoveRight`
  (params (AxisValue :type "Float (single-precision)"))
  (`PrimitiveComponent.SetPhysicsLinearVelocity` (`self.BodyMesh`) (* (`KismetMathLibrary.GetRightVector` (`self.K2_GetActorRotation`)) (* AxisValue 30.0)) true "None"))

(event `InputAxis|LookUp`
  (params (AxisValue :type "Float (single-precision)"))
  (`self.K2_AddActorLocalRotation` (`KismetMathLibrary.MakeRot` AxisValue)))

(event `InputAxis|Turn`
  (params (AxisValue :type "Float (single-precision)"))
  (`self.K2_AddActorLocalRotation` (`KismetMathLibrary.MakeRot` 0.0 AxisValue)))

(fn `UserConstructionScript`)